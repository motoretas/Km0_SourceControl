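; In-world menu actor for 360 video playback that switches camera views and controls play/pause, seeking and volume.
; It links three widget menus to itself, spawns the video spheres and binds media textures through dynamic materials.
; Two video players alternate on camera changes, with timelines fading the second sphere's opacity.
; A third player supplies continuous audio and the reference time for syncing video, using file paths from the game instance.
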(event Custom|DisableBtns
  ;[1 1 1] Disable
  (Default|DisableBtnA (Variables|Default|GetAs%20WBP%20Video%20Menu%20A))
  (Default|DisableBtnB (Variables|Default|GetAs%20WBP%20Video%20Menu%20B))
  (Default|DisableBtnPlayer (Variables|Default|GetAs%20WBP%20Video%20Menu%20Player)))

(event Custom|EnableBtns
  ;[1 1 1] Disable
  (Default|EnableBtnA (Variables|Default|GetAs%20WBP%20Video%20Menu%20A))
  (Default|EnableBtnB (Variables|Default|GetAs%20WBP%20Video%20Menu%20B))
  (Default|EnableBtnPlayer (Variables|Default|GetAs%20WBP%20Video%20Menu%20Player)))

(event Custom|BtnCameraClick
  (params (SelectedId :type Integer))
  (bind _path_0 (Variables|Default|GetPath_0))
  (Variables|Default|SetConvertedId SelectedId)
  (CallFunction|DisableBtns)
  ;[1 1 1] Media Player 01
  (if (Variables|Default|GetbIs2_Visible)
    (Class|FileMediaSource|SetFilePath (Variables|Default|GetMS_1) (Utilities|Array|Get(acopy) (Variables|/Game/Km0MonCasteller/Core/GameInstance/GI_CustomGameInstance.GI_CustomGameInstance_C|GetCollaSelNomsUrl (Variables|Default|GetAs%20GI%20Custom%20Game%20Instance)) (Variables|Default|GetConvertedId)))
    (bind _returnvalue (Media|MediaPlayer|OpenSource (Variables|Default|GetMP_1_FW) (Variables|Default|GetMediaSource_1)))
    (if _returnvalue
      (Utilities|FlowControl|Delay 0.1)
      (Variables|Default|SetCurrent%20Time (Class|MediaPlayer|GetTime (Variables|Default|GetMP_3_Audio_FW)))
      (Media|MediaPlayer|Seek (Variables|Default|GetMP_1_FW) (Variables|Default|GetCurrent%20Time))
      (Media|MediaPlayer|Play (Variables|Default|GetMP_1_FW) :!class /Script/MediaAssets.MediaPlayer)
      (bind _newtrack_0 (Timeline|Timeline_0 ReverseFromEnd)
        (:Update
          (Rendering|Material|SetScalarParameterValue (Variables|Default|GetDynMat_MP_2) "Opacity" _newtrack_0 :!class /Script/Engine.MaterialInstanceDynamic))
        (:Finished
          (Utilities|FlowControl|Delay 0.1)
          ;[1 1 1] Comment
          (Class|FileMediaSource|SetFilePath (Variables|Default|GetMS_2) _path_0)
          (bind _returnvalue_2 (Media|MediaPlayer|OpenSource (Variables|Default|GetMP_2_FW) (Variables|Default|GetMediaSource_2)))
          (if _returnvalue_2
            (Utilities|FlowControl|Delay 0.1)
            (bind _returnvalue_3 (Media|MediaPlayer|Play (Variables|Default|GetMP_2_FW) :!class /Script/MediaAssets.MediaPlayer))
            (if _returnvalue_3
              (Sequencer|Player|Pause (Variables|Default|GetMP_2_FW))
              (CallFunction|EnableBtns)
              (Variables|Default|SetbIs2_Visible false)
              (else
                (Development|PrintString "NOPE"))))))
      (else
        (Development|PrintString "NOT OPENED" true true "(R=1.000000,G=0.000000,B=0.002506,A=1.000000)")))
    (else
      ;[1 1 1] Media Player 01
      (Class|FileMediaSource|SetFilePath (Variables|Default|GetMS_2) (Utilities|Array|Get(acopy) (Variables|/Game/Km0MonCasteller/Core/GameInstance/GI_CustomGameInstance.GI_CustomGameInstance_C|GetCollaSelNomsUrl (Variables|Default|GetAs%20GI%20Custom%20Game%20Instance)) (Variables|Default|GetConvertedId)))
      (bind _returnvalue_4 (Media|MediaPlayer|OpenSource (Variables|Default|GetMP_2_FW) (Variables|Default|GetMediaSource_2)))
      (if _returnvalue_4
        (Utilities|FlowControl|Delay 0.1)
        (Variables|Default|SetCurrent%20Time (Class|MediaPlayer|GetTime (Variables|Default|GetMP_3_Audio_FW)))
        (Media|MediaPlayer|Seek (Variables|Default|GetMP_2_FW) (Variables|Default|GetCurrent%20Time))
        (Media|MediaPlayer|Play (Variables|Default|GetMP_2_FW) :!class /Script/MediaAssets.MediaPlayer)
        (bind _newtrack_0_2 (Timeline|Tl_0-1_1_BtoA PlayFromStart)
          (:Update
            (Rendering|Material|SetScalarParameterValue (Variables|Default|GetDynMat_MP_2) "Opacity" _newtrack_0_2 :!class /Script/Engine.MaterialInstanceDynamic))
          (:Finished
            (Utilities|FlowControl|Delay 0.1)
            ;[1 1 1] Comment
            (Class|FileMediaSource|SetFilePath (Variables|Default|GetMS_1) _path_0)
            (bind _returnvalue_5 (Media|MediaPlayer|OpenSource (Variables|Default|GetMP_1_FW) (Variables|Default|GetMediaSource_1)))
            (if _returnvalue_5
              (Utilities|FlowControl|Delay 0.1)
              (bind _returnvalue_6 (Media|MediaPlayer|Play (Variables|Default|GetMP_1_FW) :!class /Script/MediaAssets.MediaPlayer))
              (if _returnvalue_6
                (Sequencer|Player|Pause (Variables|Default|GetMP_1_FW))
                (CallFunction|EnableBtns)
                (Variables|Default|SetbIs2_Visible true)
                (else
                  (Development|PrintString "NOPE")))
              (else
                (Development|PrintString "NOT OPE N")))))
        (else
          (Development|PrintString "NOT OPENED" true true "(R=1.000000,G=0.000000,B=0.002506,A=1.000000)"))))))

(event Custom|BtnPlayerClick
  (params (PlayerId :type Integer))
  (bind _mp_3_audio_fw (Variables|Default|GetMP_3_Audio_FW))
  (bind _returnvalue (Media|MediaPlayer|GetDuration _mp_3_audio_fw))
  (Variables|Default|SetPlayer%20Id PlayerId)
  (switch int PlayerId
    (:0
      (Utilities|FlowControl|FlipFlop
        (:A
          ;[1 1 1] PAUSE
          (if (Variables|Default|GetbIs2_Visible)
            (Sequencer|Player|Pause (Variables|Default|GetMP_2_FW))
            (else
              (Sequencer|Player|Pause (Variables|Default|GetMP_1_FW))))
          (Sequencer|Player|Pause (Variables|Default|GetMP_3_Audio_FW))
          (Default|SwitchPlayPauseBtn (Variables|Default|GetAs%20WBP%20Video%20Menu%20Player) true))
        (:B
          ;[1 1 1] PLAY
          (if (Variables|Default|GetbIs2_Visible)
            (Media|MediaPlayer|Play (Variables|Default|GetMP_2_FW) :!class /Script/MediaAssets.MediaPlayer)
            (else
              (Media|MediaPlayer|Play (Variables|Default|GetMP_1_FW) :!class /Script/MediaAssets.MediaPlayer)))
          (Media|MediaPlayer|Play (Variables|Default|GetMP_3_Audio_FW) :!class /Script/MediaAssets.MediaPlayer)
          (Default|SwitchPlayPauseBtn (Variables|Default|GetAs%20WBP%20Video%20Menu%20Player) false))))
    (:2
      ;[1 1 1] REWIND 7
      (Variables|Default|SetCurrent%20Time (Class|MediaPlayer|GetTime (Variables|Default|GetMP_3_Audio_FW)))
      (if (< (Math|Timespan|MakeTimespan 0) (- (Variables|Default|GetCurrent%20Time) (Math|Timespan|MakeTimespan 0 0 0 (Variables|Default|GetSecondsJumpForward))))
        (Development|PrintString (Utilities|String|ToString(Integer) (Math|Timespan|GetSeconds (- (Variables|Default|GetCurrent%20Time) (Math|Timespan|MakeTimespan 0 0 0 (Variables|Default|GetSecondsJumpForward))))) true true "(R=1.000000,G=0.065528,B=0.000000,A=1.000000)" 4.0)
        (Variables|Default|SetCurrent%20Time (- (Variables|Default|GetCurrent%20Time) (Math|Timespan|MakeTimespan 0 0 0 (Variables|Default|GetSecondsJumpForward))))
        (else
          (Variables|Default|SetCurrent%20Time (Math|Timespan|MakeTimespan 0))))
      (if (Variables|Default|GetbIs2_Visible) :!label _label
        (bind _returnvalue_2 (Sequencer|Player|Pause (Variables|Default|GetMP_3_Audio_FW)))
        (bind _returnvalue_3 (Sequencer|Player|Pause (Variables|Default|GetMP_2_FW)))
        (if (and _returnvalue_3 _returnvalue_2)
          (bind _returnvalue_4 (Media|MediaPlayer|Seek (Variables|Default|GetMP_3_Audio_FW) (Variables|Default|GetCurrent%20Time)))
          (bind _returnvalue_5 (Media|MediaPlayer|Seek (Variables|Default|GetMP_2_FW) (Variables|Default|GetCurrent%20Time)))
          (if (and _returnvalue_5 _returnvalue_4)
            (Utilities|FlowControl|Delay 0.1)
            (Media|MediaPlayer|Play (Variables|Default|GetMP_2_FW) :!class /Script/MediaAssets.MediaPlayer)
            (Media|MediaPlayer|Play (Variables|Default|GetMP_3_Audio_FW) :!class /Script/MediaAssets.MediaPlayer)))
        (else
          (bind _returnvalue_6 (Sequencer|Player|Pause (Variables|Default|GetMP_1_FW)))
          (bind _returnvalue_7 (Sequencer|Player|Pause (Variables|Default|GetMP_3_Audio_FW)))
          (if (and _returnvalue_6 _returnvalue_7)
            (bind _returnvalue_8 (Media|MediaPlayer|Seek (Variables|Default|GetMP_1_FW) (Variables|Default|GetCurrent%20Time)))
            (bind _returnvalue_9 (Media|MediaPlayer|Seek (Variables|Default|GetMP_3_Audio_FW) (Variables|Default|GetCurrent%20Time)))
            (if (and _returnvalue_8 _returnvalue_9)
              (Utilities|FlowControl|Delay 0.1)
              (bind _returnvalue_10 (Media|MediaPlayer|Play (Variables|Default|GetMP_1_FW) :!class /Script/MediaAssets.MediaPlayer))
              (if _returnvalue_10
                (bind _returnvalue_11 (Media|MediaPlayer|Play (Variables|Default|GetMP_3_Audio_FW) :!class /Script/MediaAssets.MediaPlayer))
                (if _returnvalue_11
                  _)))))))
    (:3
      ;[1 1 1] FFW 6
      (Variables|Default|SetCurrent%20Time (Class|MediaPlayer|GetTime (Variables|Default|GetMP_3_Audio_FW)))
      (if (> _returnvalue (+ (Math|Timespan|MakeTimespan 0 0 0 (Variables|Default|GetSecondsJumpForward)) (Variables|Default|GetCurrent%20Time)))
        (Variables|Default|SetCurrent%20Time (+ (Math|Timespan|MakeTimespan 0 0 0 (Variables|Default|GetSecondsJumpForward)) (Variables|Default|GetCurrent%20Time)))
        (Development|PrintString (Utilities|String|ToString(Integer) (Math|Timespan|GetSeconds (+ (Math|Timespan|MakeTimespan 0 0 0 (Variables|Default|GetSecondsJumpForward)) (Variables|Default|GetCurrent%20Time)))))
        (goto _label)
        (else
          (Variables|Default|SetCurrent%20Time (- _returnvalue (Math|Timespan|MakeTimespan 0 0 0 5)))
          (if true
            (bind _returnvalue_12 (Media|MediaPlayer|Seek (Variables|Default|GetMP_3_Audio_FW) (Variables|Default|GetCurrent%20Time)))
            (bind _returnvalue_13 (Media|MediaPlayer|Seek (Variables|Default|GetMP_2_FW) (Variables|Default|GetCurrent%20Time)))
            (if (and _returnvalue_13 _returnvalue_12)
              (Utilities|FlowControl|Delay 0.1)
              (Media|MediaPlayer|Play (Variables|Default|GetMP_2_FW) :!class /Script/MediaAssets.MediaPlayer)
              (Media|MediaPlayer|Play (Variables|Default|GetMP_3_Audio_FW) :!class /Script/MediaAssets.MediaPlayer)
              (Utilities|FlowControl|Delay 0.1)
              (Sequencer|Player|Pause (Variables|Default|GetMP_3_Audio_FW))
              (Sequencer|Player|Pause (Variables|Default|GetMP_2_FW)))
            (else
              (bind _returnvalue_14 (Media|MediaPlayer|Seek (Variables|Default|GetMP_1_FW) (Variables|Default|GetCurrent%20Time)))
              (bind _returnvalue_15 (Media|MediaPlayer|Seek (Variables|Default|GetMP_3_Audio_FW) (Variables|Default|GetCurrent%20Time)))
              (if (and _returnvalue_14 _returnvalue_15)
                (Utilities|FlowControl|Delay 0.1)
                (bind _returnvalue_16 (Media|MediaPlayer|Play (Variables|Default|GetMP_1_FW) :!class /Script/MediaAssets.MediaPlayer))
                (if _returnvalue_16
                  (bind _returnvalue_17 (Media|MediaPlayer|Play (Variables|Default|GetMP_3_Audio_FW) :!class /Script/MediaAssets.MediaPlayer))
                  (if _returnvalue_17
                    (Utilities|FlowControl|Delay 0.1)
                    (EventDispatchers|AssignOnEndReached (Variables|Default|GetMP_3_Audio_FW) (delegate Custom|OnEndReached_Event_0))))))))))
    (:4
      ;[1 1 1] VOL  DOWN -
      (bind _output_get (Variables|Default|SetVolumeMultiplier%20MP03%202 (|(clamp((x+step),0,1)) (stale _output_get) -0.1)))
      (Development|PrintString (Utilities|String|ToString(Float) (|(clamp((x+step),0,1)) _output_get -0.1)))
      (if (== 0.0 (|(clamp((x+step),0,1)) _output_get -0.1))
        (Default|SwitchVolDown (Variables|Default|GetAs%20WBP%20Video%20Menu%20Player))
        (else
          (Default|SwitchVolDown (Variables|Default|GetAs%20WBP%20Video%20Menu%20Player) 1)
          (Class|MediaPlayer|SetNativeVolume (Variables|Default|GetMP_3_Audio_FW) (|(clamp((x+step),0,1)) _output_get -0.1)))))
    (:5
      ;[1 1 1] volume up
      (bind _output_get_2 (Variables|Default|SetVolumeMultiplier%20MP03%202 (|(clamp((x+step),0,1)) (stale _output_get_2) 0.1)))
      (Development|PrintString (Utilities|String|ToString(Float) (|(clamp((x+step),0,1)) _output_get_2 0.1)))
      (if (== 1.0 (|(clamp((x+step),0,1)) _output_get_2 0.1))
        (Default|SwitchVolUp (Variables|Default|GetAs%20WBP%20Video%20Menu%20Player))
        (else
          (Default|SwitchVolUp (Variables|Default|GetAs%20WBP%20Video%20Menu%20Player) 1)
          (Class|MediaPlayer|SetNativeVolume (Variables|Default|GetMP_3_Audio_FW) (|(clamp((x+step),0,1)) _output_get_2 0.1)))))))

(event Custom|OnEndReached_Event_0
  (Sequencer|Player|Pause (Variables|Default|GetMP_1_FW))
  (bind _returnvalue (Sequencer|Player|Pause (Variables|Default|GetMP_3_Audio_FW)))
  (if _returnvalue
    _))

(event EventBeginPlay
  (Utilities|FlowControl|Sequence
    (:then_0
      ;[1 1 1] ANDROID
      (Class|MediaPlayer|SetNativeVolume (Variables|Default|GetMP_3_Audio_FW) 0.7))
    (:then_1
      ;[1 1 1] COLLA ID
      (bind _asgi_custom_game_instance (Utilities|Casting|CastToGI_CustomGameInstance (Game|GetGameInstance)))
      (bind _output_get (Variables|Default|SetAs%20GI%20Custom%20Game%20Instance _asgi_custom_game_instance))
      (Default|SetSelectedIdUrl _output_get (Variables|Default|GetColla%20ID)))
    (:then_2
      ;[1 1 1] cast menu A
      (bind _aswbp_video_menu_a (Utilities|Casting|CastToWBP_VideoMenuA (UserInterface|GetUserWidgetObject (Variables|Default|GetWidget_VideoMenuA))))
      (bind _output_get_2 (Variables|Default|SetAs%20WBP%20Video%20Menu%20A _aswbp_video_menu_a))
      (Variables|/Game/Km0MonCasteller/Video/WBP_VideoMenuA.WBP_VideoMenuA_C|SetBp_VideoMenu _output_get_2 self)
      ;[1 1 1] PLAYER REF
      (bind _aswbp_video_menu_player (Utilities|Casting|CastToWBP_VideoMenuPlayer (UserInterface|GetUserWidgetObject (Variables|Default|GetWidget_VideoMenuPlayer))))
      (bind _output_get_3 (Variables|Default|SetAs%20WBP%20Video%20Menu%20Player _aswbp_video_menu_player))
      (Variables|/Game/Km0MonCasteller/Video/WBP_VideoMenuPlayer.WBP_VideoMenuPlayer_C|SetBp_VideoMenu _output_get_3 self)
      ;[1 1 1] MENU B
      (bind _aswbp_video_menu_b (Utilities|Casting|CastToWBP_VideoMenuB (UserInterface|GetUserWidgetObject (Variables|Default|GetWidget_VideoMenuB))))
      (bind _output_get_4 (Variables|Default|SetAs%20WBP%20Video%20Menu%20B _aswbp_video_menu_b))
      (Variables|/Game/Km0MonCasteller/Video/WBP_VideoMenuB.WBP_VideoMenuB_C|SetBp_VideoMenu _output_get_4 self))
    (:then_3
      ;[1 1 1] SPAWN
      (bind _returnvalue (Game|SpawnActorfromClass "/Game/Km0MonCasteller/Video/BP_360Spheres_Video.BP_360Spheres_Video_C" (Variables|Default|GetSpawn%20Transform) "AlwaysSpawn" 0 0))
      ;[1 1 1] set refs
      (Variables|Default|SetS%20MP%201 (Variables|/Game/Km0MonCasteller/Video/BP_360Spheres_Video.BP_360Spheres_Video_C|Gets_MP_1 _returnvalue))
      (Variables|Default|SetS%20MP%202 (Variables|/Game/Km0MonCasteller/Video/BP_360Spheres_Video.BP_360Spheres_Video_C|Gets_MP_2 _returnvalue))
      (Variables|Default|SetS%20MS%203 (Variables|/Game/Km0MonCasteller/Video/BP_360Spheres_Video.BP_360Spheres_Video_C|Gets_MS_3 _returnvalue))
      ;[1 1 1] DYMANIC MATERIALS
      (bind _returnvalue_2 (Rendering|Material|CreateDynamicMaterialInstance (Variables|Default|GetS%20MP%201) 0 (Rendering|Material|GetMaterial (Variables|Default|GetS%20MP%201) 0) "None" :!class /Script/Engine.PrimitiveComponent))
      (bind _output_get_5 (Variables|Default|SetDynMat_MP_1 _returnvalue_2))
      (Rendering|Material|SetTextureParameterValue _output_get_5 "T_Mplayer" (Variables|Default|GetT_MPlayer_1))
      (bind _returnvalue_3 (Rendering|Material|CreateDynamicMaterialInstance (Variables|Default|GetS%20MP%202) 0 (Rendering|Material|GetMaterial (Variables|Default|GetS%20MP%202) 0) "None" :!class /Script/Engine.PrimitiveComponent))
      (bind _output_get_6 (Variables|Default|SetDynMat_MP_2 _returnvalue_3))
      (Rendering|Material|SetTextureParameterValue _output_get_6 "T_Mplayer" (Variables|Default|GetT_MPlayer_2))
      (bind _returnvalue_4 (Rendering|Material|CreateDynamicMaterialInstance (Variables|Default|GetS%20MS%203) 0 (Rendering|Material|GetMaterial (Variables|Default|GetS%20MS%203) 0) "None" :!class /Script/Engine.PrimitiveComponent))
      (bind _output_get_7 (Variables|Default|SetDynMat_MS_3 _returnvalue_4))
      (Rendering|Material|SetTextureParameterValue _output_get_7 "T_Mplayer" (Variables|Default|GetT_MPlayer_3Audio))
      (Utilities|FlowControl|Sequence
        (:then_0
          ;[1 1 1] Media Player 01
          (Class|FileMediaSource|SetFilePath (Variables|Default|GetMS_1) (Utilities|Array|Get(acopy) (Variables|/Game/Km0MonCasteller/Core/GameInstance/GI_CustomGameInstance.GI_CustomGameInstance_C|GetCollaSelNomsUrl (Variables|Default|GetAs%20GI%20Custom%20Game%20Instance))))
          (bind _returnvalue_5 (Media|MediaPlayer|OpenSource (Variables|Default|GetMP_1_FW) (Variables|Default|GetMediaSource_1)))
          (if _returnvalue_5
            (Utilities|FlowControl|Delay 0.2)
            (Media|MediaPlayer|Play (Variables|Default|GetMP_1_FW) :!class /Script/MediaAssets.MediaPlayer)
            (else
              (Development|PrintString "NOT OPENED" true true "(R=1.000000,G=0.000000,B=0.002506,A=1.000000)"))))
        (:then_1
          ;[1 1 1] Media Player 01
          (Class|FileMediaSource|SetFilePath (Variables|Default|GetMS_3) (Utilities|Array|Get(acopy) (Variables|/Game/Km0MonCasteller/Core/GameInstance/GI_CustomGameInstance.GI_CustomGameInstance_C|GetCollaSelNomsUrl (Variables|Default|GetAs%20GI%20Custom%20Game%20Instance)) 4))
          (Media|MediaPlayer|OpenSource (Variables|Default|GetMP_3_Audio_FW) (Variables|Default|GetMediaSource_3))
          (if true
            (Utilities|FlowControl|Delay 0.2)
            (Media|MediaPlayer|Play (Variables|Default|GetMP_3_Audio_FW) :!class /Script/MediaAssets.MediaPlayer)
            (else
              (Development|PrintString "NOT OPENED" true true "(R=1.000000,G=0.000000,B=0.002506,A=1.000000)"))))))))

(fn ConstructionScript)