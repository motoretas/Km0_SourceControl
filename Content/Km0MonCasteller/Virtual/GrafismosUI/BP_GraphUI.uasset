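; Actor that hosts the animated infographic widgets (structure, pinya, weights, height, pom de dalt) for the virtual casteller graphics.
; On BeginPlay it registers with GI_CustomGameInstance's OnStartAnimGraph, caches each widget component's user widget and passes itself to it.
; The event prints the GraphId and calls StartAnimGraph on the matching widget, ignoring IsStarting.
; Graph 5's setup is disconnected, so its switch case uses an unassigned reference.
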(event `self.ReceiveBeginPlay`
  ;[1 1 1] COLLA ID
  (bind _asgi_custom_game_instance (cast `/Game/Km0MonCasteller/Core/GameInstance/GI_CustomGameInstance` (`GameplayStatics.GetGameInstance`)))
  (add `/Game/Km0MonCasteller/Core/GameInstance/GI_CustomGameInstance.OnStartAnimGraph` _asgi_custom_game_instance (delegate `OnStartAnimGraph_Event_0`))
  (`|ExecutionSequence`
    (:`then_0`
      ;[1 1 1] 1-EST
      (bind _aswbp_graph_1_estructura_ok (cast `/Game/Km0MonCasteller/Virtual/GrafismosUI/WBP_Graph_1_Estructura_OK` (`WidgetComponent.GetUserWidgetObject` (`self.Widget-1_Est`))))
      (bind _output_get (set `self.As WBP Graph 1 Estructura OK` _aswbp_graph_1_estructura_ok))
      (set `/Game/Km0MonCasteller/Virtual/GrafismosUI/WBP_Graph_1_Estructura_OK.BP_GraphUi` self _output_get))
    (:`then_1`
      ;[1 1 1] 2-EST
      (bind _aswbp_graph_2_pinya_ok (cast `/Game/Km0MonCasteller/Virtual/GrafismosUI/WBP_GRAPH_2_PINYA_OK` (`WidgetComponent.GetUserWidgetObject` (`self.Widget-2-Pinya`))))
      (bind _output_get_2 (set `self.As WBP GRAPH 2 PINYA OK` _aswbp_graph_2_pinya_ok))
      (set `/Game/Km0MonCasteller/Virtual/GrafismosUI/WBP_GRAPH_2_PINYA_OK.BP_GraphUi` self _output_get_2))
    (:`then_2`
      ;[1 1 1] 3-EST
      (bind _aswbp_graph_3_pinya_vent (cast `/Game/Km0MonCasteller/Virtual/GrafismosUI/WBP_GRAPH_3_PINYA_VENT` (`WidgetComponent.GetUserWidgetObject` (`self.Widget-3_Vent`))))
      (bind _output_get_3 (set `self.As WBP GRAPH 3 PINYA VENT` _aswbp_graph_3_pinya_vent))
      (set `/Game/Km0MonCasteller/Virtual/GrafismosUI/WBP_GRAPH_3_PINYA_VENT.BP_GraphUi` self _output_get_3))
    (:`then_4`
      ;[1 1 1] 6-PES
      (bind _aswbp_graph_6_pesos_ok (cast `/Game/Km0MonCasteller/Virtual/GrafismosUI/WBP_Graph_6_PESOS_OK` (`WidgetComponent.GetUserWidgetObject` (`self.Widget-6_Pesos`))))
      (bind _output_get_4 (set `self.As WBP Graph 6 PESOS OK` _aswbp_graph_6_pesos_ok))
      (set `/Game/Km0MonCasteller/Virtual/GrafismosUI/WBP_Graph_6_PESOS_OK.BP_GraphUi` self _output_get_4))
    (:`then_5`
      ;[1 1 1] 7-PES_TRONC
      (bind _aswbp_graph_7_pesos_b_ok (cast `/Game/Km0MonCasteller/Virtual/GrafismosUI/WBP_Graph_7_PESOS_B_OK` (`WidgetComponent.GetUserWidgetObject` (`self.Widget-7_TRONC_PES`))))
      (bind _output_get_5 (set `self.As WBP Graph 7 PESOS B OK` _aswbp_graph_7_pesos_b_ok))
      (set `/Game/Km0MonCasteller/Virtual/GrafismosUI/WBP_Graph_7_PESOS_B_OK.BP_GraphUi` self _output_get_5))
    (:`then_6`
      ;[1 1 1] 10-ALCADsa
      (bind _aswbp_graph_10_alcada_ok (cast `/Game/Km0MonCasteller/Virtual/GrafismosUI/WBP_Graph_10_ALCADA_OK` (`WidgetComponent.GetUserWidgetObject` (`self.Widget-10_ALCADA`))))
      (bind _output_get_6 (set `self.As WBP Graph 10 ALCADA OK` _aswbp_graph_10_alcada_ok))
      (set `/Game/Km0MonCasteller/Virtual/GrafismosUI/WBP_Graph_10_ALCADA_OK.BP_GraphUi` self _output_get_6))
    (:`then_7`
      ;[1 1 1] 11-ENX
      (bind _aswbp_graph_11_pomdedalt_ok (cast `/Game/Km0MonCasteller/Virtual/GrafismosUI/WBP_Graph_11_POMDEDALT_OK` (`WidgetComponent.GetUserWidgetObject` (`self.Widget-11-ENXA`))))
      (bind _output_get_7 (set `self.As WBP Graph 11 POMDEDALT OK` _aswbp_graph_11_pomdedalt_ok))
      (set `/Game/Km0MonCasteller/Virtual/GrafismosUI/WBP_Graph_11_POMDEDALT_OK.BP_GraphUi` self _output_get_7))))

(event `OnStartAnimGraph_Event_0`
  (params (GraphId :type Integer) (isStarting :type Boolean))
  ;[1 1 1] COLLA ID
  (`KismetSystemLibrary.PrintString` (`KismetStringLibrary.Conv_IntToString` GraphId) true true (struct :`G` 1.0 :`B` 0.305734 :`A` 1.0))
  (switch `int` GraphId
    (:`1`
      (`/Game/Km0MonCasteller/Virtual/GrafismosUI/WBP_Graph_1_Estructura_OK.StartAnimGraph` (`self.As WBP Graph 1 Estructura OK`)))
    (:`2`
      (`/Game/Km0MonCasteller/Virtual/GrafismosUI/WBP_GRAPH_2_PINYA_OK.StartAnimGraph` (`self.As WBP GRAPH 2 PINYA OK`)))
    (:`3`
      (`/Game/Km0MonCasteller/Virtual/GrafismosUI/WBP_GRAPH_3_PINYA_VENT.StartAnimGraph` (`self.As WBP GRAPH 3 PINYA VENT`)))
    (:`5`
      (`/Game/Km0MonCasteller/Virtual/GrafismosUI/WBP_GRAPH_5_PINYA_FORMATGETS.StartAnimGraph` (`self.As WBP GRAPH 5 PINYA FORMATGETS`)))
    (:`6`
      (`/Game/Km0MonCasteller/Virtual/GrafismosUI/WBP_Graph_6_PESOS_OK.StartAnimGraph` (`self.As WBP Graph 6 PESOS OK`)))
    (:`7`
      (`/Game/Km0MonCasteller/Virtual/GrafismosUI/WBP_Graph_7_PESOS_B_OK.StartAnimGraph` (`self.As WBP Graph 7 PESOS B OK`)))
    (:`10`
      (`/Game/Km0MonCasteller/Virtual/GrafismosUI/WBP_Graph_10_ALCADA_OK.StartAnimGraph` (`self.As WBP Graph 10 ALCADA OK`)))
    (:`11`
      (`/Game/Km0MonCasteller/Virtual/GrafismosUI/WBP_Graph_11_POMDEDALT_OK.StartAnimGraph` (`self.As WBP Graph 11 POMDEDALT OK`)))))

(fn `UserConstructionScript`)