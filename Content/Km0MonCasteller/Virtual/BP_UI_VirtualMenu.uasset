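; Virtual menu actor for 360-degree image viewing, linking two menu widgets to a spawned BP_360Sphere_Virtual.
; A button click disables both menus, selects textures by ID and crossfades the sphere's dynamic material through OpacityAtoB timelines.
; Image B fades in, then after a delay image A takes over by fade or snap, depending on the two-image and faded-image flags.
; A previous faded image is faded out first, and buttons re-enable when the sequence ends.
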(event `self.ReceiveBeginPlay`
  ;[1 1 1] Set REF BP on Virt A
  (bind _aswbp_virtual_menu_a (cast `/Game/Km0MonCasteller/Virtual/WBP_VirtualMenuA` (`WidgetComponent.GetUserWidgetObject` (`self.Widget_VirtualA`))))
  (bind _output_get (set `self.As WBP Virtual Menu A` _aswbp_virtual_menu_a))
  (set `/Game/Km0MonCasteller/Virtual/WBP_VirtualMenuA.BP_VirtualMenu` self _output_get)
  ;[1 1 1] Set REF BP on Virt B
  (bind _aswbp_virtual_menu_b (cast `/Game/Km0MonCasteller/Virtual/WBP_VirtualMenuB` (`WidgetComponent.GetUserWidgetObject` (`self.Widget_VirtualB`))))
  (bind _output_get_2 (set `self.As WBP Virtual Menu B` _aswbp_virtual_menu_b))
  (set `/Game/Km0MonCasteller/Virtual/WBP_VirtualMenuB.BP_VirtualMenu` self _output_get_2)
  (bind _returnvalue (`|SpawnActorFromClass` "/Game/Km0MonCasteller/Virtual/BP_360Sphere_Virtual.BP_360Sphere_Virtual_C" (`self.Spawn Transform_0`) "AlwaysSpawn" "OverrideRootScale" null null))
  (bind _virtualsphere (`/Game/Km0MonCasteller/Virtual/BP_360Sphere_Virtual.VirtualSphere` _returnvalue))
  (bind _returnvalue_2 (`PrimitiveComponent.CreateDynamicMaterialInstance` _virtualsphere 0 (`PrimitiveComponent.GetMaterial` _virtualsphere 0) "None"))
  (set `self.DynamicMaterialInstanceVirtual` _returnvalue_2))

(event `Disable_BTNS`
  (params (`bIsAorB?` :type Boolean))
  (`/Game/Km0MonCasteller/Virtual/WBP_VirtualMenuA.DisableBtnA` (`self.As WBP Virtual Menu A`))
  (`/Game/Km0MonCasteller/Virtual/WBP_VirtualMenuB.DisableBtnB` (`self.As WBP Virtual Menu B`)))

(event `Enable_BTNS`
  (`/Game/Km0MonCasteller/Virtual/WBP_VirtualMenuA.EnableBtnA` (`self.As WBP Virtual Menu A`))
  (`/Game/Km0MonCasteller/Virtual/WBP_VirtualMenuB.EnableBtnB` (`self.As WBP Virtual Menu B`)))

(event `BtnClick`
  (params (SelectedId :type Integer) (Has2Images :type Boolean) (HasFadedImage :type Boolean))
  (set `self.Has 2Images` Has2Images)
  (set `self.Has Faded Image` HasFadedImage)
  (set `self.ConvertedId` (+ SelectedId 1))
  ;[1 1 1] Disable BTNS
  (`/Game/Km0MonCasteller/Virtual/WBP_VirtualMenuA.DisableBtnA` (`self.As WBP Virtual Menu A`))
  (`/Game/Km0MonCasteller/Virtual/WBP_VirtualMenuB.DisableBtnB` (`self.As WBP Virtual Menu B`))
  (if (`self.PrevHadFadedImage`)
    (`KismetSystemLibrary.PrintString` "FADING OUT ")
    (bind (_direction _newtrack_0) (`Timeline|Tl_0-02_1` :`NewTime` 1.0 :!via `ReverseFromEnd`)
      (:`Update`
        (`MaterialInstanceDynamic.SetScalarParameterValue` (`self.DynamicMaterialInstanceVirtual`) "OpacityAtoB" _newtrack_0))
      (:`Finished`
        (bind _output_get (set `self.Texture B` (select `int` (`self.ConvertedId`) :`0` (`self.Texture_0`) :`1` (`self.T_1A`) :`2` (`self.T_2A`) :`3` (`self.T_3A`) :`4` (`self.T_4A`) :`5` (`self.T_5A`) :`6` (`self.T_6A`) :`7` (`self.T_7A`) :`8` (`self.T_8A`) :`9` (`self.T_9A`) :`10` (`self.T_10A`) :`11` (`self.T_11A`)) :!label _label))
        (`MaterialInstanceDynamic.SetTextureParameterValue` (`self.DynamicMaterialInstanceVirtual`) "DT_360Virt_B" _output_get)
        (bind (_direction_2 _newtrack_0_2) (`Timeline|Tl_0-1_1` :`NewTime` 1.0 :!via `PlayFromStart`)
          (:`Update`
            (`MaterialInstanceDynamic.SetScalarParameterValue` (`self.DynamicMaterialInstanceVirtual`) "OpacityAtoB" _newtrack_0_2))
          (:`Finished`
            (`KismetSystemLibrary.PrintString` "IMAGE B VISIBLE" true true (struct :`R` 1.0 :`G` 0.010362 :`B` 0.020309 :`A` 1.0) 4.0)
            (`KismetSystemLibrary.Delay` 2.0)
            (bind _output_get_2 (set `self.Texture A` (select `int` (`self.ConvertedId`) :`0` (`self.Texture_0`) :`1` (`self.T_1B`) :`2` (`self.T_2B`) :`3` (`self.T_3B`) :`4` (`self.T_4B`) :`5` (`self.T_5B`) :`6` (`self.T_6B`) :`7` (`self.T_7B`) :`8` (`self.T_8B`) :`9` (`self.T_9B`) :`10` (`self.T_10B`) :`11` (`self.T_11`))))
            (`MaterialInstanceDynamic.SetTextureParameterValue` (`self.DynamicMaterialInstanceVirtual`) "DT_360Virt_A" _output_get_2)
            (if (`self.Has 2Images`)
              (if (`self.Has Faded Image`)
                (bind (_direction_3 _newtrack_0_3) (`Timeline|Tl_02-1_1` :`NewTime` 1.0 :!via `ReverseFromEnd`)
                  (:`Update`
                    (`MaterialInstanceDynamic.SetScalarParameterValue` (`self.DynamicMaterialInstanceVirtual`) "OpacityAtoB" _newtrack_0_3))
                  (:`Finished`
                    (`KismetSystemLibrary.PrintString` "HAS FADED IMAGE" true true (struct :`R` 1.0 :`G` 0.075413 :`A` 1.0))
                    (set `self.PrevHadFadedImage` true)
                    (`KismetSystemLibrary.PrintString` "END" true true (struct :`R` 1.0 :`G` 1.0 :`B` 1.0 :`A` 1.0) 4.0 :!label _label_2)
                    (`self.Enable_BTNS`)))
                (else
                  (bind (_direction_4 _newtrack_0_4) (`Timeline|Tl_01_1_B` :`NewTime` 1.0 :!via `ReverseFromEnd`)
                    (:`Update`
                      (`MaterialInstanceDynamic.SetScalarParameterValue` (`self.DynamicMaterialInstanceVirtual`) "OpacityAtoB" _newtrack_0_4))
                    (:`Finished`
                      (`KismetSystemLibrary.PrintString` "HAS 2 IMAGES")
                      (set `self.PrevHadFadedImage` false)
                      (goto _label_2)))))
              (else
                (`KismetSystemLibrary.PrintString` "NO 2 IMAGES")
                (`MaterialInstanceDynamic.SetScalarParameterValue` (`self.DynamicMaterialInstanceVirtual`) "OpacityAtoB" 0.0)
                (`KismetSystemLibrary.Delay` 0.2)
                (set `self.PrevHadFadedImage` false)
                (goto _label_2)))))))
    (else
      (goto _label))))

(fn `UserConstructionScript`)