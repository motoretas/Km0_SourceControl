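; BP_UI_Menu is a menu actor that sequences animated widget panels and ends by fading out to open a level.
; BeginPlay casts its widget components' widgets to two menus and logo panels, handing each a back-reference.
; ClickBtnMenu stores CollaID and runs numbered steps: intro, submenu, second menu, then reversed animations and a delayed pawn fade.
; Both right-logo variants are cast from WidgetMenuRight; the END variant is re-cast when invalid.
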(event `self.ReceiveBeginPlay`
  ;[1 1 1] MA
  (bind _aswbp_menu_a (cast `/Game/Km0MonCasteller/Menu/WBP_MenuA` (`WidgetComponent.GetUserWidgetObject` (`self.Widget_MenuA`))))
  (bind _output_get (set `self.As WBP Menu A` _aswbp_menu_a))
  (set `/Game/Km0MonCasteller/Menu/WBP_MenuA.BP_UI_Menu` self _output_get)
  ;[1 1 1] Comment
  (bind _aswbp_menu_b (cast `/Game/Km0MonCasteller/Menu/WBP_MenuB` (`WidgetComponent.GetUserWidgetObject` (`self.Widget_MenuB`))))
  (bind _output_get_2 (set `self.As WBP Menu B` _aswbp_menu_b))
  (set `/Game/Km0MonCasteller/Menu/WBP_MenuB.BP_UI_Menu` self _output_get_2)
  ;[1 1 1] Comment
  (bind _aswbp_menu_logo_left (cast `/Game/Km0MonCasteller/Menu/WBP_MenuLogoLeft` (`WidgetComponent.GetUserWidgetObject` (`self.Widget_MenuLeft`))))
  (bind _output_get_3 (set `self.As WBP Menu Logo Left` _aswbp_menu_logo_left))
  (set `/Game/Km0MonCasteller/Menu/WBP_MenuLogoLeft.BP_UI_Menu` self _output_get_3)
  ;[1 1 1] Comment
  (bind _aswbp_menu_logo_right (cast `/Game/Km0MonCasteller/Menu/WBP_MenuLogoRight` (`WidgetComponent.GetUserWidgetObject` (`self.Widget_MenuRight`))))
  (bind _output_get_4 (set `self.As WBP Menu Logo Right` _aswbp_menu_logo_right))
  (set `/Game/Km0MonCasteller/Menu/WBP_MenuLogoRight.BP_UI_Menu` self _output_get_4)
  ;[1 1 1] Comment
  (bind _aswbp_menu_logo_right_end (cast `/Game/Km0MonCasteller/Menu/WBP_MenuLogoRightEND` (`WidgetComponent.GetUserWidgetObject` (`self.Widget_MenuRight`))))
  (bind _output_get_5 (set `self.As WBP Menu Logo Right END` _aswbp_menu_logo_right_end))
  (set `/Game/Km0MonCasteller/Menu/WBP_MenuLogoRightEND.BP_UI_Menu` self _output_get_5))

(event `ClickBtnMenu`
  (params (AnimPasos :type Integer) (CollaID :type Boolean))
  (bind _as_wbp_menu_a (`self.As WBP Menu A`))
  (bind _as_wbp_menu_logo_right_end (`self.As WBP Menu Logo Right END`))
  (bind _as_wbp_menu_logo_right (`self.As WBP Menu Logo Right`))
  (bind _as_wbp_menu_logo_left (`self.As WBP Menu Logo Left`))
  (bind _as_wbp_menu_logo_right_2 (`self.As WBP Menu Logo Right`))
  (bind _as_wbp_menu_b (`self.As WBP Menu B`))
  (bind _as_wbp_menu_a_2 (`self.As WBP Menu A`))
  (bind _as_wbp_menu_a_3 (`self.As WBP Menu A`))
  (bind _as_wbp_menu_logo_right_end_2 (`self.As WBP Menu Logo Right END`))
  (bind _as_wbp_menu_b_2 (`self.As WBP Menu B`))
  (bind _as_wbp_menu_a_4 (`self.As WBP Menu A`))
  (bind _as_wbp_menu_logo_left_2 (`self.As WBP Menu Logo Left`))
  (set `self.Colla ID` CollaID)
  (switch `int` AnimPasos
    (:`0`
      ;[1 1 1] PASO 0
      (`UserWidget.PlayAnimation` _as_wbp_menu_a_4 (`/Game/Km0MonCasteller/Menu/WBP_MenuA.Intro` _as_wbp_menu_a_4) 0.0 1 "Forward" (`self.MenuAnimPlaybackSpeed`) false)
      (`KismetSystemLibrary.Delay` (/ 1.5 (`self.MenuAnimPlaybackSpeed`)))
      (`UserWidget.PlayAnimation` _as_wbp_menu_logo_left_2 (`/Game/Km0MonCasteller/Menu/WBP_MenuLogoLeft.Intro` _as_wbp_menu_logo_left_2) 0.0 1 "Forward" (`self.MenuAnimPlaybackSpeed`) false)
      (`KismetSystemLibrary.Delay` (/ 0.5 (`self.MenuAnimPlaybackSpeed`)))
      (`UserWidget.PlayAnimation` _as_wbp_menu_logo_right_2 (`/Game/Km0MonCasteller/Menu/WBP_MenuLogoRight.Intro` _as_wbp_menu_logo_right_2) 0.0 1 "Forward" (`self.MenuAnimPlaybackSpeed`) false)
      (`KismetSystemLibrary.Delay` (/ 0.5 (`self.MenuAnimPlaybackSpeed`))))
    (:`1`
      ;[1 1 1] PASO 1
      (`UserWidget.PlayAnimation` _as_wbp_menu_a_3 (`/Game/Km0MonCasteller/Menu/WBP_MenuA.Submenu` _as_wbp_menu_a_3) 0.0 1 "Forward" (`self.MenuAnimPlaybackSpeed`) false))
    (:`2`
      ;[1 1 1] PASO 2
      (`UserWidget.PlayAnimation` _as_wbp_menu_logo_right (`/Game/Km0MonCasteller/Menu/WBP_MenuLogoRight.ChangePosition` _as_wbp_menu_logo_right) 0.0 1 "Forward" (`self.MenuAnimPlaybackSpeed`) false)
      (`KismetSystemLibrary.Delay` (/ 0.5 (`self.MenuAnimPlaybackSpeed`)))
      (`UserWidget.PlayAnimation` _as_wbp_menu_b_2 (`/Game/Km0MonCasteller/Menu/WBP_MenuB.Intro` _as_wbp_menu_b_2) 0.0 1 "Forward" (`self.MenuAnimPlaybackSpeed`) false)
      (`KismetSystemLibrary.Delay` 0.2)
      (`/Engine/EditorBlueprintResources/StandardMacros.IsValid` (`self.As WBP Menu Logo Right END`)
        (:`Is Valid`
          (`UserWidget.PlayAnimation` _as_wbp_menu_logo_right_end_2 (`/Game/Km0MonCasteller/Menu/WBP_MenuLogoRightEND.Intro` _as_wbp_menu_logo_right_end_2) 0.0 1 "Forward" (`self.MenuAnimPlaybackSpeed`) false))
        (:`Is Not Valid`
          ;[1 1 1] Comment
          (bind _aswbp_menu_logo_right_end (cast `/Game/Km0MonCasteller/Menu/WBP_MenuLogoRightEND` (`WidgetComponent.GetUserWidgetObject` (`self.Widget_MenuRight`))))
          (set `self.As WBP Menu Logo Right END` _aswbp_menu_logo_right_end))))
    (:`3`
      (`|ExecutionSequence`
        (:`then_0`
          ;[1 1 1] PASO 1
          (`UserWidget.PlayAnimation` _as_wbp_menu_b (`/Game/Km0MonCasteller/Menu/WBP_MenuB.Intro` _as_wbp_menu_b) 0.0 1 "Reverse" (`self.MenuAnimPlaybackSpeed`) false)
          (`/Engine/EditorBlueprintResources/StandardMacros.IsValid` _as_wbp_menu_logo_right_end
            (:`Is Valid`
              (`UserWidget.PlayAnimation` _as_wbp_menu_logo_right_end (`/Game/Km0MonCasteller/Menu/WBP_MenuLogoRightEND.Intro` _as_wbp_menu_logo_right_end) 0.0 1 "Reverse" 1.0 false)
              ;;[1 0.008162 0] ERROR REVISAR
              (`UserWidget.PlayAnimation` _as_wbp_menu_logo_left (`/Game/Km0MonCasteller/Menu/WBP_MenuLogoLeft.Intro` _as_wbp_menu_logo_left) 0.0 1 "Reverse" (`self.MenuAnimPlaybackSpeed`) false)
              (`UserWidget.PlayAnimation` _as_wbp_menu_a (`/Game/Km0MonCasteller/Menu/WBP_MenuA.Submenu` _as_wbp_menu_a) 0.0 1 "Reverse" (`self.MenuAnimPlaybackSpeed`) false)
              (`UserWidget.PlayAnimation` _as_wbp_menu_a_2 (`/Game/Km0MonCasteller/Menu/WBP_MenuA.Intro` _as_wbp_menu_a_2) 0.0 1 "Reverse" (`self.MenuAnimPlaybackSpeed`) false))
            (:`Is Not Valid`
              ;[1 1 1] Comment
              (bind _aswbp_menu_logo_right_end_2 (cast `/Game/Km0MonCasteller/Menu/WBP_MenuLogoRightEND` (`WidgetComponent.GetUserWidgetObject` (`self.Widget_MenuRight`))))
              (set `self.As WBP Menu Logo Right END` _aswbp_menu_logo_right_end_2))))
        (:`then_1`
          (`KismetSystemLibrary.Delay` 3.0)
          ;[1 1 1] FADE
          (message `/Game/Km0MonCasteller/Core/Interfaces/BPI_OpenLevel.FadeToBlack` (`GameplayStatics.GetPlayerPawn` 0) 2.0 (struct) true true true (`self.LevelToOpen`)))))))

(fn `UserConstructionScript`)